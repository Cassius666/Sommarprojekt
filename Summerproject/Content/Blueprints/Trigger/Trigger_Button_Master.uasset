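; Master trigger button that sinks when its box is overlapped and fires event dispatchers, in either timer or pressure mode.
; In timer mode only the player triggers it: it hands the duration to ThirdPersonCharacter's event timer, fires Timer0 at start and end, then rises, with a DoOnce blocking retriggers.
; In pressure mode any overlap begin or end fires PressureButton and lowers or raises the button.
; The construction script applies the button's material.
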(event `self.Box.OnComponentBeginOverlap`
  (params (OverlappedComponent :type "PrimitiveComponent Object Reference") (OtherActor :type "Actor Object Reference") (OtherComp :type "PrimitiveComponent Object Reference") (OtherBodyIndex :type Integer) (bFromSweep :type Boolean) (SweepResult :type "HitResult Structure (by ref)"))
  (bind _timer (`self.Timer`))
  (if (`self.TimerButton`)
    (if (`self.IsOverlappingActor` (`GameplayStatics.GetPlayerCharacter` 0))
      (`/Engine/EditorBlueprintResources/StandardMacros.DoOnce` false :!label _label
        (:`Completed`
          (`KismetSystemLibrary.MoveComponentTo` (`self.Button`) (0.0 0.0 -49.0) (struct) false false 1.0)
          (bind _asthird_person_character (cast `/Game/ThirdPersonBP/Blueprints/ThirdPersonCharacter` (`GameplayStatics.GetPlayerCharacter` 0)))
          (set `/Game/ThirdPersonBP/Blueprints/ThirdPersonCharacter.Timer_For_Events` _timer _asthird_person_character)
          (`self.Timer>0`)
          (`/Game/ThirdPersonBP/Blueprints/ThirdPersonCharacter.Event_Timer` _asthird_person_character)
          (`KismetSystemLibrary.Delay` _timer)
          (`self.Timer>0`)
          (`KismetSystemLibrary.MoveComponentTo` (`self.Button`) (0.0 0.0 -39.0) (struct) false false 1.0)
          (goto _label :!via `Reset`))))
    (else
      (`self.PressureButton`)
      (`KismetSystemLibrary.MoveComponentTo` (`self.Button`) (0.0 0.0 -49.0) (struct) false false 1.0)
      (`KismetSystemLibrary.PrintString` "ON"))))

(event `self.Box.OnComponentEndOverlap`
  (params (OverlappedComponent :type "PrimitiveComponent Object Reference") (OtherActor :type "Actor Object Reference") (OtherComp :type "PrimitiveComponent Object Reference") (OtherBodyIndex :type Integer))
  (if (not (`self.TimerButton`))
    (`self.PressureButton`)
    (`KismetSystemLibrary.MoveComponentTo` (`self.Button`) (0.0 0.0 -39.0) (struct) false false 1.0)
    (`KismetSystemLibrary.PrintString` "OFF")))

(fn `UserConstructionScript`
  (`PrimitiveComponent.SetMaterial` (`self.Button`) 0 (`self.Material`)))