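; Floor button trigger with two modes, chosen by WhichButton; begin and end overlap share the same logic.
; Timer mode plays a timeline moving the chosen water's box and a linked actor along its spline, starts the character's event timer and fires Timer0 before and after the delay.
; On/Off mode fires PressureButton and slides the button down or up with player overlap.
; Construction script applies the button material.
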(event `self.Box.OnComponentBeginOverlap`
  (params (OverlappedComponent :type "PrimitiveComponent Object Reference") (OtherActor :type "Actor Object Reference") (OtherComp :type "PrimitiveComponent Object Reference") (OtherBodyIndex :type Integer) (bFromSweep :type Boolean) (SweepResult :type "HitResult Structure (by ref)"))
  (bind _returnvalue (`GameplayStatics.GetPlayerCharacter` 0))
  (bind _button (`self.Button`))
  (bind _timer (`self.Timer`))
  (bind _waterspline (`/Game/Blueprints/Trigger/Swimming.WaterSpline` (`self.ChooseWater`)))
  (switch `/Game/Blueprints/Data/Button_List` (`self.Which_Button?`) :!label _label
    (:`NewEnumerator0`
      (if (`self.IsOverlappingActor` _returnvalue)
        (`/Engine/EditorBlueprintResources/StandardMacros.DoOnce` false :!label _label_2
          (:`Completed`
            (if (`PrimitiveComponent.IsOverlappingActor` OverlappedComponent OtherActor)
              (bind (_direction _newtrack_0) (`Timeline|Timeline_0` :!via `PlayFromStart` :!label _label_3)
                (:`Update`
                  (`SceneComponent.K2_SetWorldLocation` (`/Game/Blueprints/Trigger/Swimming.Box` (`self.ChooseWater`)) (`SplineComponent.GetLocationAtDistanceAlongSpline` _waterspline (* _newtrack_0 (`SplineComponent.GetSplineLength` _waterspline)) "World") false false)
                  (`SceneComponent.K2_SetWorldLocation` (`Actor.RootComponent` (`self.NewVar_1`)) (`SplineComponent.GetLocationAtDistanceAlongSpline` _waterspline (* _newtrack_0 (`SplineComponent.GetSplineLength` _waterspline)) "World") false false)
                  (bind _asthird_person_character (cast `/Game/ThirdPersonBP/Blueprints/ThirdPersonCharacter` (`GameplayStatics.GetPlayerCharacter` 0)))
                  (set `/Game/ThirdPersonBP/Blueprints/ThirdPersonCharacter.Timer_For_Events` _timer _asthird_person_character)
                  (`self.Timer>0`)
                  (`/Game/ThirdPersonBP/Blueprints/ThirdPersonCharacter.Event_Timer` _asthird_person_character)
                  (`KismetSystemLibrary.Delay` _timer)
                  (`self.Timer>0`)
                  (`KismetSystemLibrary.MoveComponentTo` (`self.Button`) (0.0 0.0 -39.0) (struct) false false 1.0)
                  (goto _label_2 :!via `Reset`)))
              (else
                (goto _label_3 :!via `Reverse`)))))))
    (:`NewEnumerator1`
      (`self.PressureButton`)
      (if (`PrimitiveComponent.IsOverlappingActor` OverlappedComponent _returnvalue)
        (`KismetSystemLibrary.MoveComponentTo` _button (0.0 0.0 -49.0) (struct) false false 1.0)
        (else
          (`self.PressureButton`)
          (`KismetSystemLibrary.MoveComponentTo` _button (0.0 0.0 -39.0) (struct) false false 1.0))))))

(event `self.Box.OnComponentEndOverlap`
  (params (OverlappedComponent :type "PrimitiveComponent Object Reference") (OtherActor :type "Actor Object Reference") (OtherComp :type "PrimitiveComponent Object Reference") (OtherBodyIndex :type Integer))
  (goto _label))

(fn `UserConstructionScript`
  (`PrimitiveComponent.SetMaterial` (`self.Button`) 0 (`self.Material`)))