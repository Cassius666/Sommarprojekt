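; Ladder is an interactible actor that marks a ThirdPersonCharacter as being on a ladder while it overlaps the Box volume.
; On begin overlap it passes its up vector to the character's LadderZvector, enables input for player controller 0 and sets OnLadder.
; On end overlap it clears OnLadder and restores Walking movement mode.
; The file contains no climbing movement logic of its own.
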(event `self.Box.OnComponentBeginOverlap`
  (params (OverlappedComponent :type "PrimitiveComponent Object Reference") (OtherActor :type "Actor Object Reference") (OtherComp :type "PrimitiveComponent Object Reference") (OtherBodyIndex :type Integer) (bFromSweep :type Boolean) (SweepResult :type "HitResult Structure (by ref)"))
  (bind _asthird_person_character (cast `/Game/ThirdPersonBP/Blueprints/ThirdPersonCharacter` OtherActor))
  (set `/Game/ThirdPersonBP/Blueprints/ThirdPersonCharacter.Ladder_Z-vector` (`self.GetActorUpVector`) _asthird_person_character)
  (`self.EnableInput` _asthird_person_character (`GameplayStatics.GetPlayerController` 0))
  (set `/Game/ThirdPersonBP/Blueprints/ThirdPersonCharacter.On_Ladder` true _asthird_person_character))

(event `self.Box.OnComponentEndOverlap`
  (params (OverlappedComponent :type "PrimitiveComponent Object Reference") (OtherActor :type "Actor Object Reference") (OtherComp :type "PrimitiveComponent Object Reference") (OtherBodyIndex :type Integer))
  (bind _asthird_person_character (cast `/Game/ThirdPersonBP/Blueprints/ThirdPersonCharacter` OtherActor))
  (set `/Game/ThirdPersonBP/Blueprints/ThirdPersonCharacter.On_Ladder` false _asthird_person_character)
  (`CharacterMovementComponent.SetMovementMode` (`Character.CharacterMovement` _asthird_person_character) "MOVE_Walking" 0))

(fn `UserConstructionScript`)