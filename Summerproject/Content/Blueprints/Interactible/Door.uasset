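; Interactive door that raises and lowers its Cube along relative Z in response to three linked buttons.
; On BeginPlay it binds to each button's timer and pressure events and copies the first button's material onto the Cube.
; Pressure events toggle the height through a FlipFlop.
; Timer events raise it while the player character's TimerForEvents exceeds a threshold, otherwise lower it.
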(event `CustomEvent_0`
  (bind _cube (`self.Cube`))
  (bind (_relativelocation_x _relativelocation_y) (`KismetMathLibrary.BreakVector` (`SceneComponent.RelativeLocation` (`self.Cube`))))
  (`/Engine/EditorBlueprintResources/StandardMacros.FlipFlop`
    (:`A`
      (`KismetSystemLibrary.MoveComponentTo` _cube (`KismetMathLibrary.MakeVector` _relativelocation_x _relativelocation_y 300.0)))
    (:`B`
      (`KismetSystemLibrary.MoveComponentTo` _cube (`KismetMathLibrary.MakeVector` _relativelocation_x _relativelocation_y 100.0)))))

(event `self.ReceiveBeginPlay`
  (bind _choose_button1 (`self.Choose_Button1`))
  (add `/Game/Blueprints/Trigger/Trigger_Button_Master.Timer>0` _choose_button1 (delegate `OpenDoor`))
  (add `/Game/Blueprints/Trigger/Trigger_Button_Master.Timer>0` (`self.Choose_Button2`) (delegate `OpenDoor`))
  (add `/Game/Blueprints/Trigger/Trigger_Button_Master.Timer>0` (`self.Choose_Button3`) (delegate `OpenDoor`))
  (add `/Game/Blueprints/Trigger/Trigger_Button_Master.PressureButton` _choose_button1 (delegate `CustomEvent_0`))
  (add `/Game/Blueprints/Trigger/Trigger_Button_Master.PressureButton` (`self.Choose_Button2`) (delegate `CustomEvent_0`))
  (add `/Game/Blueprints/Trigger/Trigger_Button_Master.PressureButton` (`self.Choose_Button3`) (delegate `CustomEvent_0`))
  (`PrimitiveComponent.SetMaterial` (`self.Cube`) 0 (`PrimitiveComponent.GetMaterial` (`/Game/Blueprints/Trigger/Trigger_Button_Master.Button` (`self.Choose_Button1`)) 0)))

(event `OpenDoor`
  (bind _cube (`self.Cube`))
  (bind (_relativelocation_x _relativelocation_y) (`KismetMathLibrary.BreakVector` (`SceneComponent.RelativeLocation` (`self.Cube`))))
  (bind _asthird_person_character (cast `/Game/ThirdPersonBP/Blueprints/ThirdPersonCharacter` (`GameplayStatics.GetPlayerCharacter` 0)))
  (if (> (`/Game/ThirdPersonBP/Blueprints/ThirdPersonCharacter.Timer_For_Events` _asthird_person_character) 1.0)
    (`KismetSystemLibrary.MoveComponentTo` _cube (`KismetMathLibrary.MakeVector` _relativelocation_x _relativelocation_y 300.0))
    (else
      (`KismetSystemLibrary.MoveComponentTo` _cube (`KismetMathLibrary.MakeVector` _relativelocation_x _relativelocation_y 100.0)))))

(fn `UserConstructionScript`)