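; Interactible box that slides one fixed step along X or Y when the player character overlaps one of its side triggers.
; Four overlap events each move the Cube component in one of the four horizontal directions with a short MoveComponentTo.
; A shared Moving flag, per-direction DoOnce nodes and a delay slightly longer than the move block new pushes until the current one finishes.
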(event `self.Side X+.OnComponentBeginOverlap`
  (params (OverlappedComponent :type "PrimitiveComponent Object Reference") (OtherActor :type "Actor Object Reference") (OtherComp :type "PrimitiveComponent Object Reference") (OtherBodyIndex :type Integer) (bFromSweep :type Boolean) (SweepResult :type "HitResult Structure (by ref)"))
  (bind (_relativelocation_x _relativelocation_y _relativelocation_z) (`KismetMathLibrary.BreakVector` (`SceneComponent.RelativeLocation` (`self.Cube`))))
  (if (and (not (`self.Moving?`)) (`PrimitiveComponent.IsOverlappingActor` OverlappedComponent (`GameplayStatics.GetPlayerCharacter` 0)))
    (set `self.Moving?` true)
    (`/Engine/EditorBlueprintResources/StandardMacros.DoOnce` false :!label _label
      (:`Completed`
        (`KismetSystemLibrary.MoveComponentTo` (`self.Cube`) (`KismetMathLibrary.MakeVector` (+ _relativelocation_x -100.0) _relativelocation_y _relativelocation_z) (struct) false false 0.5)
        (`KismetSystemLibrary.Delay` 0.6)
        (set `self.Moving?` false)
        (goto _label :!via `Reset`)))))

(event `self.Side X-.OnComponentBeginOverlap`
  (params (OverlappedComponent :type "PrimitiveComponent Object Reference") (OtherActor :type "Actor Object Reference") (OtherComp :type "PrimitiveComponent Object Reference") (OtherBodyIndex :type Integer) (bFromSweep :type Boolean) (SweepResult :type "HitResult Structure (by ref)"))
  (bind (_relativelocation_x _relativelocation_y _relativelocation_z) (`KismetMathLibrary.BreakVector` (`SceneComponent.RelativeLocation` (`self.Cube`))))
  (if (and (not (`self.Moving?`)) (`PrimitiveComponent.IsOverlappingActor` OverlappedComponent (`GameplayStatics.GetPlayerCharacter` 0)))
    (set `self.Moving?` true)
    (`/Engine/EditorBlueprintResources/StandardMacros.DoOnce` false :!label _label_2
      (:`Completed`
        (`KismetSystemLibrary.MoveComponentTo` (`self.Cube`) (`KismetMathLibrary.MakeVector` (+ _relativelocation_x 100.0) _relativelocation_y _relativelocation_z) (struct) false false 0.5)
        (`KismetSystemLibrary.Delay` 0.6)
        (set `self.Moving?` false)
        (goto _label_2 :!via `Reset`)))))

(event `self.Side Y+.OnComponentBeginOverlap`
  (params (OverlappedComponent :type "PrimitiveComponent Object Reference") (OtherActor :type "Actor Object Reference") (OtherComp :type "PrimitiveComponent Object Reference") (OtherBodyIndex :type Integer) (bFromSweep :type Boolean) (SweepResult :type "HitResult Structure (by ref)"))
  (bind (_relativelocation_x _relativelocation_y _relativelocation_z) (`KismetMathLibrary.BreakVector` (`SceneComponent.RelativeLocation` (`self.Cube`))))
  (if (and (not (`self.Moving?`)) (`PrimitiveComponent.IsOverlappingActor` OverlappedComponent (`GameplayStatics.GetPlayerCharacter` 0)))
    (set `self.Moving?` true)
    (`/Engine/EditorBlueprintResources/StandardMacros.DoOnce` false :!label _label_3
      (:`Completed`
        (`KismetSystemLibrary.MoveComponentTo` (`self.Cube`) (`KismetMathLibrary.MakeVector` _relativelocation_x (+ _relativelocation_y -100.0) _relativelocation_z) (struct) false false 0.5)
        (`KismetSystemLibrary.Delay` 0.6)
        (set `self.Moving?` false)
        (goto _label_3 :!via `Reset`)))))

(event `self.Side Y-.OnComponentBeginOverlap`
  (params (OverlappedComponent :type "PrimitiveComponent Object Reference") (OtherActor :type "Actor Object Reference") (OtherComp :type "PrimitiveComponent Object Reference") (OtherBodyIndex :type Integer) (bFromSweep :type Boolean) (SweepResult :type "HitResult Structure (by ref)"))
  (bind (_relativelocation_x _relativelocation_y _relativelocation_z) (`KismetMathLibrary.BreakVector` (`SceneComponent.RelativeLocation` (`self.Cube`))))
  (if (and (not (`self.Moving?`)) (`PrimitiveComponent.IsOverlappingActor` OverlappedComponent (`GameplayStatics.GetPlayerCharacter` 0)))
    (set `self.Moving?` true)
    (`/Engine/EditorBlueprintResources/StandardMacros.DoOnce` false :!label _label_4
      (:`Completed`
        (`KismetSystemLibrary.MoveComponentTo` (`self.Cube`) (`KismetMathLibrary.MakeVector` _relativelocation_x (+ _relativelocation_y 100.0) _relativelocation_z) (struct) false false 0.5)
        (`KismetSystemLibrary.Delay` 0.6)
        (set `self.Moving?` false)
        (goto _label_4 :!via `Reset`)))))

(fn `UserConstructionScript`)